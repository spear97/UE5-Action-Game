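; Lightsaber actor with a Niagara blade that activates on spawn and can be picked up by the player through Interact.
; Each tick while active, InitBlade line-traces along the scaled forward vector, sets the beam end to the full trace length, and shows an impact effect at any blocking hit.
; Pickup flags the third-person character as equipped, attaches the saber to its right-hand socket and activates it.
; Helper functions toggle visibility and recolor both effects.
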(event EventBeginPlay
  ;[1 1 1] Activate Upon being Spawned in World
  (CallFunction|Activate))

(event EventTick
  (params (DeltaSeconds :type Float%20%28single-precision%29))
  ;[1 1 1] Update the Blade for each frame
  (CallFunction|InitBlade))

(event EventInteract
  ;[1 1 1] When Player Interacts attempt to Pickup
  (CallFunction|PlayPickup))

(fn ConstructionScript)

(fn Deactivate
  ;[1 1 1] When Blade is not active Hide both the Blade and the Impact Effect
  (bind _output_get (Variables|Default|SetActive? false))
  (Rendering|SetVisibility (Variables|Default|GetNiagaraLaser) _output_get false))

(fn Activate
  ;[1 1 1] When Blade is active Hide both the Blade and the Impact Effect
  (bind _output_get (Variables|Default|SetActive? true))
  (Rendering|SetVisibility (Variables|Default|GetNiagaraLaser) _output_get false))

(fn SetColor
  (params (Param :type Linear%20Color%20Structure))
  ;[1 1 1] Set the Color of the Blade and the Impact Effect to a particular color
  (Effects|Components|ParticleSystem|SetColorParameter (Variables|Default|GetNiagaraLaser) "Color" Param))

(fn InitBlade
  (bind _returnvalue (Transformation|GetActorLocation))
  (bind _niagaralaserimpact (Variables|Default|GetNiagaraLaserImpact))
  ;[1 1 1] When active, Calculate the end point for the blade and the position where the impact effect should spawn
  (if (Variables|Default|GetActive?)
    (bind _output_get (Variables|Default|SetTraceEnd (+ _returnvalue (* (* (Transformation|GetActorForwardVector) (Variables|Default|Getdirection)) (Variables|Default|Getdistance)))))
    (bind _outhit (Collision|LineTraceByChannel _returnvalue _output_get "TraceTypeQuery2" false (Utilities|Array|MakeArray (Game|GetPlayerCharacter 0)) "None"))
    (Variables|Default|SetHit (.bblockinghit _outhit))
    (Variables|Default|SetHitLocation (.location _outhit))
    (Effects|Components|ParticleSystem|SetVectorParameter (Variables|Default|GetNiagaraLaser) "LaserEnd" (Variables|Default|GetTraceEnd))
    (Rendering|SetVisibility _niagaralaserimpact (Variables|Default|GetHit) false)
    (Transformation|SetWorldLocation _niagaralaserimpact (Variables|Default|GetHitLocation) false false)))

(fn PlayPickup
  (Variables|/Game/ThirdPerson/Blueprints/BP_ThirdPersonCharacter.BP_ThirdPersonCharacter_C|SetLightSaberEquipped? (.AsBP%20Third%20Person%20Character (Utilities|Casting|CastToBP_ThirdPersonCharacter (Game|GetPlayerCharacter 0))) true)
  (Development|PrintString "Hello There!")
  (Transformation|AttachComponentToComponent (Variables|/Script/Engine.Character|GetMesh (.AsBP%20Third%20Person%20Character (Utilities|Casting|CastToBP_ThirdPersonCharacter (Game|GetPlayerCharacter 0)))) "LightSaber_Socket_R" "SnapToTarget" "SnapToTarget" "KeepRelative" true)
  (CallFunction|Activate))