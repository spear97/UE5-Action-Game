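; Laser actor that draws a Niagara beam with an impact effect, purely visual in this graph.
; BeginPlay tints both effects, then each Tick line-traces on the Camera channel along the actor's up vector scaled by Direction.
; The trace sets the beam end and places the impact effect, shown only on a blocking hit.
; Beam length snaps to the hit distance and extends over time up to a cap, so it grows gradually.
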(event EventBeginPlay
  (Effects|Components|ParticleSystem|SetColorParameter (Variables|Default|GetNiagaraLaser) "Color" "(R=0.013702,G=0.024158,B=0.048172,A=1.000000)"))

(event EventTick
  (params (DeltaSeconds :type Float%20%28single-precision%29))
  (bind _returnvalue (Transformation|GetActorLocation))
  (bind _niagaralaserimpact (Variables|Default|GetNiagaraLaserImpact))
  (Utilities|FlowControl|Sequence
    (:then_0
      (bind _output_get (Variables|Default|SetTraceEnd (+ _returnvalue (* (* (Transformation|GetActorUpVector) (Variables|Default|Getdirection)) (Variables|Default|Getdistance)))))
      (bind _outhit (Collision|LineTraceByChannel _returnvalue _output_get "TraceTypeQuery2" false 0 "None"))
      (Variables|Default|SetHit (.bblockinghit _outhit))
      (Variables|Default|SetHitLocation (.location _outhit))
      (Effects|Components|ParticleSystem|SetVectorParameter (Variables|Default|GetNiagaraLaser) "LaserEnd" (select (Variables|Default|GetHit) (Variables|Default|GetHitLocation) (Variables|Default|GetTraceEnd)))
      (Rendering|SetVisibility _niagaralaserimpact (Variables|Default|GetHit) false)
      (Transformation|SetWorldLocation _niagaralaserimpact (Variables|Default|GetHitLocation) false false)
      (if (Variables|Default|GetHit)
        (Variables|Default|Setdistance (Math|Vector|VectorLength (- (Variables|Default|GetHitLocation) (Transformation|GetActorLocation))))))
    (:then_1
      (if (< (Variables|Default|Getdistance) 5e+03)
        (Variables|Default|Setdistance (+ (Variables|Default|Getdistance) (* DeltaSeconds 2e+03)))))))

(fn ConstructionScript)